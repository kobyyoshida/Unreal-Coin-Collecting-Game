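; Collectable coin actor that spins in place and is picked up on overlap.
; On any actor overlap it casts player 0's HUD to TPgameHUD, calls Collected on it and destroys itself.
; Tick adds frame-rate-independent yaw by rebuilding the whole transform, which also zeroes roll and pitch and forces unit scale.
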(event `self.ReceiveActorBeginOverlap`
  (params (OtherActor :type "Actor Object Reference"))
  ;[1 1 1] Collecting Coin
  (bind _astpgame_hud (cast `/Game/Blueprints/TPgame/TPgameHUD` (`PlayerController.GetHUD` (`GameplayStatics.GetPlayerController` 0))))
  (bind _output_get (set `self.collectibleGameHUD` _astpgame_hud))
  (`/Game/Blueprints/TPgame/TPgameHUD.collected` _output_get)
  (`self.K2_DestroyActor`))

(event `self.ReceiveTick`
  (params (DeltaSeconds :type "Float (single-precision)"))
  ;[1 1 1] Rotater
  (`self.K2_SetActorTransform` (`KismetMathLibrary.MakeTransform` (`self.K2_GetActorLocation`) (`KismetMathLibrary.MakeRotator` 0.0 0.0 (+ (* DeltaSeconds 100.0) (.yaw (`self.K2_GetActorRotation`)))))))

(fn `UserConstructionScript`)